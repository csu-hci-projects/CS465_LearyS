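; Reaction-timer cube that measures how long it takes to be overlapped after turning red, reporting results as debug prints.
; Ending an overlap starts a random timer that turns the cube red, records the time and increments the test count.
; Beginning an overlap turns it blue after a retriggerable delay, then updates an incremental running average with the elapsed time, which includes that delay.
; Several disconnected test snippets remain in the graph.
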(event `self.ReceiveBeginPlay`
  ;[1 1 1] when start, pring to debug for visual seperation
  (`KismetSystemLibrary.PrintString` "Start Test"))

(event `self.ReceiveTick`
  (params (DeltaSeconds :type "Float (single-precision)")))

(event `self.ReceiveActorBeginOverlap`
  (params (OtherActor :type "Actor Object Reference"))
  (bind _avgeventtime (`self.AvgEventTime`))
  ;[1 1 1] When Pressed, shift to blue(Neutral) and calculate time delta and running average
  (`KismetSystemLibrary.RetriggerableDelay` 0.5)
  (`PrimitiveComponent.SetMaterial` (`self.CubeMesh`) 0 "/Engine/VREditor/BasicMeshes/MI_Cube_02.MI_Cube_02")
  (if (not (== (`self.TotalTests`) 0))
    (bind _output_get (set `self.TimeOfBlueShift` (`KismetSystemLibrary.GetGameTimeInSeconds`)))
    (bind _output_get_2 (set `self.Delta` (- _output_get (`self.TimeOfRedShift`))))
    (`KismetSystemLibrary.PrintString` (`KismetStringLibrary.Conv_DoubleToString` _output_get_2))
    (`KismetSystemLibrary.PrintString` "Delta Above")
    (bind _output_get_3 (set `self.AvgEventTime` (+ (/ (- (`self.Delta`) _avgeventtime) (`self.TotalTests`)) _avgeventtime)))
    (`KismetSystemLibrary.PrintString` (`KismetStringLibrary.Conv_DoubleToString` _output_get_3))
    (`KismetSystemLibrary.PrintString` "Above New Average")))

(event `self.ReceiveActorEndOverlap`
  (params (OtherActor :type "Actor Object Reference"))
  ;[1 1 1] When no longer pressed, set a random 2-10 second timer and shift back to red, then add 1 to tests total for average calculation
  (`KismetSystemLibrary.K2_SetTimerDelegate` (delegate `Trigger material shift`) (`KismetMathLibrary.RandomFloatInRange` 2.0 10.0)))

(event `Trigger material shift`
  ;[1 1 1] When no longer pressed, set a random 2-10 second timer and shift back to red, then add 1 to tests total for average calculation
  (`PrimitiveComponent.SetMaterial` (`self.CubeMesh`) 0 "/Engine/VREditor/BasicMeshes/MI_Cube_03.MI_Cube_03")
  (set `self.TimeOfRedShift` (`KismetSystemLibrary.GetGameTimeInSeconds`))
  (if (== (`self.TotalTests`) 0)
    (set `self.TotalTests` (+ (`self.TotalTests`) 1))
    (`KismetSystemLibrary.PrintString` "First Switch to Red")
    (else
      (set `self.TotalTests` (+ (`self.TotalTests`) 1)))))

(fn `UserConstructionScript`)